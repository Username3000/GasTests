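; Gameplay ability that keeps a character's movement in sync with its Gameplay Ability System state.
; On activation it caches the owning Character and its movement component, then starts persistent async listeners.
; An attribute-change listener writes the new value to MaxWalkSpeed.
; Adding the State.CantMove tag makes the controller ignore move input, and removing it clears that block.
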(event Custom|BindWalkSpeed
  (bind _newvalue (Ability|Tasks|WaitForAttributeChanged (Variables|Default|GetCharacter) "(AttributeName=\"WalkSpeed\",Attribute=/Script/GasTests.CharacterBasis_AS:WalkSpeed,AttributeOwner=/Script/CoreUObject.Class'\"/Script/GasTests.CharacterBasis_AS\"')")
    (:Changed
      (Variables|/Script/Engine.CharacterMovementComponent|SetMaxWalkSpeed (Variables|Default|GetMovementComponent) _newvalue))))

(event Custom|BindMovement
  (Utilities|FlowControl|Sequence
    (:then_0
      (Ability|Tasks|WaitGameplayTagAdd "(TagName=\"State.CantMove\")" 0
        (:Added
          (Input|SetIgnoreMoveInput (Pawn|GetController (Variables|Default|GetCharacter)) true))))
    (:then_1
      (Ability|Tasks|WaitGameplayTagRemove "(TagName=\"State.CantMove\")" 0
        (:Removed
          (Input|SetIgnoreMoveInput (Pawn|GetController (Variables|Default|GetCharacter)) false))))))

(event Ability|EventActivateAbility
  (bind _returnvalue (Ability|GetActorInfo))
  (bind (_owneractor _movementcomponent) (Utilities|Struct|BreakGameplayAbilityActorInfo _returnvalue))
  (bind _ascharacter (Utilities|Casting|CastToCharacter _owneractor))
  (Variables|Default|SetCharacter _ascharacter)
  (bind _ascharacter_movement_component (Utilities|Casting|CastToCharacterMovementComponent _movementcomponent))
  (Variables|Default|SetMovementComponent _ascharacter_movement_component)
  (CallFunction|BindWalkSpeed)
  (CallFunction|BindMovement))