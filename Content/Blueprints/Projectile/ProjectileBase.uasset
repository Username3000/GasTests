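; Base projectile actor that applies a damage effect to whatever it strikes, then destroys itself.
; On BeginPlay it copies Speed into the ProjectileMovement component and activates it.
; Both actor overlaps and Sphere hits feed a shared Hit function, which ignores the Instigator.
; Hit applies DamageEffect through the target's MyAbilitySystemComponent, crediting the Instigator's controller, and destroys the projectile even when the target lacks that component.
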(event OnComponentHit(Sphere)
  (params (HitComponent :type Primitive%20Component%20Object%20Reference) (OtherActor :type Actor%20Object%20Reference) (OtherComp :type Primitive%20Component%20Object%20Reference) (NormalImpulse :type Vector :default "0, 0, 0") (Hit :type Hit%20Result%20Structure%20%28by%20ref%29))
  (CallFunction|Hit OtherActor))

(event EventBeginPlay
  (Variables|/Script/Engine.ProjectileMovementComponent|SetMaxSpeed (Variables|Default|GetProjectileMovement) (Variables|Settings|GetSpeed))
  (Variables|/Script/Engine.ProjectileMovementComponent|SetInitialSpeed (Variables|Default|GetProjectileMovement) (Variables|Settings|GetSpeed))
  (Components|Activation|Activate (Variables|Default|GetProjectileMovement) false))

(event Collision|EventActorBeginOverlap
  (params (OtherActor :type Actor%20Object%20Reference))
  (CallFunction|Hit OtherActor))

(fn ConstructionScript)

(fn Hit
  (params (OtherActor :type Actor%20Object%20Reference))
  (if (!= OtherActor (Variables|Actor|GetInstigator))
    (Utilities|FlowControl|Sequence
      (:then_0
        (bind _asmy_ability_system_component (Utilities|Casting|CastToMyAbilitySystemComponent (Ability|GetAbilitySystemComponent OtherActor)))
        (Class|MyAbilitySystemComponent|ApplyDamageEffect _asmy_ability_system_component (Variables|Settings|GetDamageEffect) 0.0 (Pawn|GetController (Variables|Actor|GetInstigator))))
      (:then_1
        (Actor|DestroyActor)))))